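; BP_Player is the player actor, which jumps on Space and ends the run when it is destroyed.
; On BeginPlay it caches the bp_MainGame game instance, binds its death handler to OnDestroyed and resets the score to zero.
; The death handler raises the high score if beaten, saves through the game instance and opens the MainMenu level.
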(event `Key|SpaceBar`
  (params (Key :type "Key Structure"))
  (:`Pressed`
    (`self.Jump`)))

(event `self.ReceiveBeginPlay`
  (bind _asbp_main_game (cast `/Game/Blueprints/bp_MainGame` (`GameplayStatics.GetGameInstance`)))
  (set `self.gameInstance` _asbp_main_game)
  (add `self.OnDestroyed` (delegate `death`))
  (set `/Game/Blueprints/bp_MainGame.score` 0 (`self.gameInstance`)))

(event `death` :!signature `self.OnDestroyed`
  (params (DestroyedActor :type "Actor Object Reference"))
  (bind _gameinstance (`self.gameInstance`))
  (bind _score (`/Game/Blueprints/bp_MainGame.score` _gameinstance))
  (if (> _score (`/Game/Blueprints/bp_MainGame.highscore` _gameinstance))
    (set `/Game/Blueprints/bp_MainGame.highscore` _score _gameinstance))
  (`/Game/Blueprints/bp_MainGame.Save` (`self.gameInstance`))
  (`GameplayStatics.OpenLevel` "MainMenu"))

(fn `UserConstructionScript`)