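; Enemy spawner actor that keeps spawning walking or flying enemies at random intervals.
; BeginPlay starts a timer for spawnEnemy, which re-arms itself with a random delay after each spawn.
; A random modulo check picks a walker about one time in three, otherwise a flyer.
; Spawns take X, Y and rotation from the Cube component, with height set by a separate arrow component for each type.
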(event `spawnEnemy`
  (bind _returnvalue (`SceneComponent.K2_GetComponentToWorld` (`self.Cube`)))
  (bind _returnvalue_2 (`SceneComponent.K2_GetComponentToWorld` (`self.Cube`)))
  (bind (_returnvalue_x _returnvalue_y _returnvalue_z) (`KismetMathLibrary.BreakVector` (`SceneComponent.K2_GetComponentLocation` (`self.BottomArrow`))))
  (if (== (mod (`KismetMathLibrary.RandomIntegerInRange` 1 100) 3) 0)
    (`|SpawnActorFromClass` "/Game/Blueprints/walkingEnemy.walkingEnemy_C" (`KismetMathLibrary.MakeTransform` (`KismetMathLibrary.MakeVector` (.x (.location _returnvalue)) (.y (.location _returnvalue)) (.z (.location (`SceneComponent.K2_GetComponentToWorld` (`self.walkerArrow`))))) (.rotation _returnvalue)) "Undefined" "MultiplyWithRoot" null null)
    (else
      (`|SpawnActorFromClass` "/Game/Blueprints/flyingEnemy.flyingEnemy_C" (`KismetMathLibrary.MakeTransform` (`KismetMathLibrary.MakeVector` (.x (.location _returnvalue_2)) (.y (.location _returnvalue_2)) _returnvalue_z) (.rotation _returnvalue_2)) "Undefined" "MultiplyWithRoot" null null)))
  (`KismetSystemLibrary.K2_SetTimer` null "spawnEnemy" (`KismetMathLibrary.RandomFloatInRange` 1.0 5.0)))

(event `self.ReceiveBeginPlay`
  (`KismetSystemLibrary.K2_SetTimer` null "spawnEnemy" 3.0))

(fn `UserConstructionScript`)