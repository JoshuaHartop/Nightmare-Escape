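; bp_MainGame handles high score persistence through custom Save and Load events.
; Save creates a GameSave object if none is valid, copies Highscore into it and writes it to the "savedgame" slot.
; Load reads that slot if it exists, or creates a new GameSave otherwise, then copies the object's Highscore back into the Blueprint.
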(event `Save`
  (bind _savegame (`self.saveGame`))
  (`/Engine/EditorBlueprintResources/StandardMacros.IsValid` _savegame
    (:`Is Valid`
      _)
    (:`Is Not Valid`
      (bind _returnvalue (`GameplayStatics.CreateSaveGameObject` "/Game/Blueprints/gameSave.gameSave_C"))
      (set `self.saveGame` _returnvalue)))
  (set `/Game/Blueprints/gameSave.highscore` (`self.highscore`) _savegame)
  (`GameplayStatics.SaveGameToSlot` (`self.saveGame`) "savedgame"))

(event `Load`
  (bind _returnvalue (`GameplayStatics.DoesSaveGameExist` "savedgame"))
  (if _returnvalue
    (bind _returnvalue_2 (`GameplayStatics.LoadGameFromSlot` "savedgame"))
    (bind _asgame_save (cast `/Game/Blueprints/gameSave` _returnvalue_2))
    (set `self.saveGame` _asgame_save)
    (else
      (bind _returnvalue_3 (`GameplayStatics.CreateSaveGameObject` "/Game/Blueprints/gameSave.gameSave_C"))
      (set `self.saveGame` _returnvalue_3)))
  (set `self.highscore` (`/Game/Blueprints/gameSave.highscore` (`self.saveGame`))))